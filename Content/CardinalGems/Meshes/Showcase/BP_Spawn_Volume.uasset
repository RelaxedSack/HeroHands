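; Showcase spawner that fills its Volume box with randomized Dynamic_Gem_Spawn actors while the Spawn input is held.
; Input press and release open and close a gate fed by Tick, with a short Delay throttling the spawn rate.
; Each gem gets random rotation, per-axis scale and an offset within the box extents, added to actor location without applying the volume's rotation.
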(event EventBeginPlay)

(event EventActorBeginOverlap
  (params (OtherActor :type Actor%20Object%20Reference)))

(event EventTick
  (params (DeltaSeconds :type Float%20%28single-precision%29))
  (bind _returnvalue (Math|Random|RandomFloatinRange 0.3 1.2))
  (bind _volume (Variables|Default|GetVolume))
  (bind _returnvalue_2 (Components|Box|GetScaledBoxExtent _volume))
  (bind (_x _y _z) (Math|Vector|BreakVector _returnvalue_2))
  (Utilities|FlowControl|Gate true
    (:Exit
      (Utilities|FlowControl|Delay 0.05)
      (Game|SpawnActorfromClass "/Game/CardinalGems/Meshes/Showcase/Dynamic_Gem_Spawn.Dynamic_Gem_Spawn_C" (Math|Transform|MakeTransform (+ (Math|Vector|MakeVector (Math|Random|RandomFloatinRange (* _x -1.0) _x) (Math|Random|RandomFloatinRange (* _y -1.0) _y) (Math|Random|RandomFloatinRange (* _z -1.0) _z)) (Transformation|GetActorLocation)) (Math|Random|RandomRotator true) (Math|Vector|MakeVector _returnvalue _returnvalue _returnvalue)) "Undefined" 0 0))))

(event Input|ActionEvents|InputActionSpawn
  (params (Key :type Key%20Structure :default "AnyKey"))
  (bind _returnvalue (Math|Random|RandomFloatinRange 0.3 1.2))
  (bind _volume (Variables|Default|GetVolume))
  (bind _returnvalue_2 (Components|Box|GetScaledBoxExtent _volume))
  (bind (_x _y _z) (Math|Vector|BreakVector _returnvalue_2))
  (:Pressed
    (Utilities|FlowControl|Gate true) ; enters at Open
  )
  (:Released
    (Utilities|FlowControl|Gate true) ; enters at Close
  ))

(fn ConstructionScript)