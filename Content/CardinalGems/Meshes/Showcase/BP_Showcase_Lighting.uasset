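; BP_Showcase_Lighting is a lighting rig Blueprint for the CardinalGems mesh showcase, built from nine spotlight components.
; The construction script applies one shared SidesIntensity value to eight of the spotlights and a separate TopIntensity to SpotLight4.
; The event graph holds only disabled placeholder events, so the Blueprint adds no runtime behavior.
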(event EventBeginPlay)

(event EventActorBeginOverlap
  (params (OtherActor :type Actor%20Object%20Reference)))

(event EventTick
  (params (DeltaSeconds :type Float%20%28single-precision%29)))

(fn ConstructionScript
  (Rendering|Components|Light|SetIntensity (Variables|Default|GetSpotLight1) (Variables|Default|GetSides%20Intensity))
  (Rendering|Components|Light|SetIntensity (Variables|Default|GetSpotLight4) (Variables|Default|GetTop%20Intensity)))