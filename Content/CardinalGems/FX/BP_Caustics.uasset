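; BP_Caustics is a gem FX actor that projects caustic patterns using three cone lights for red, green and blue channels.
; The construction script sets each channel's visibility, color and multiplied intensity, plus shared shadow, attenuation and cone angle settings.
; A PickCaustic selector can swap each light's function material to an alternate caustic set, giving each channel its own material instance.
; All setup runs at construction, with no active runtime logic.
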(event EventBeginPlay)

(event EventActorBeginOverlap
  (params (OtherActor :type Actor%20Object%20Reference)))

(event EventTick
  (params (DeltaSeconds :type Float%20%28single-precision%29)))

(fn ConstructionScript
  (Rendering|SetVisibility (Variables|Default|GetLight_RED) (Variables|Default|GetR) false)
  (Rendering|SetVisibility (Variables|Default|GetLight_GREEN) (Variables|Default|GetG) false)
  (Rendering|SetVisibility (Variables|Default|GetLIGHT_Blue) (Variables|Default|GetB) false)
  (Rendering|Components|Light|SetCastShadows (Variables|Default|GetLight_RED) (Variables|Default|GetCast%20Shadows))
  (Rendering|Components|Light|SetIntensity (Variables|Default|GetLight_RED) (* (Variables|Default|GetR_Intensity) (Variables|Default|GetIntensity%20Multiplier)))
  (Rendering|Components|Light|SetIntensity (Variables|Default|GetLight_GREEN) (* (Variables|Default|GetG_Intensity) (Variables|Default|GetIntensity%20Multiplier)))
  (Rendering|Components|Light|SetIntensity (Variables|Default|GetLIGHT_Blue) (* (Variables|Default|GetB_Intensity) (Variables|Default|GetIntensity%20Multiplier)))
  (Rendering|Components|Light|SetLightColor (Variables|Default|GetLight_RED) (Variables|Default|GetR_Color) true)
  (Rendering|Components|Light|SetLightColor (Variables|Default|GetLight_GREEN) (Variables|Default|GetG_Color) true)
  (Rendering|Components|Light|SetLightColor (Variables|Default|GetLIGHT_Blue) (Variables|Default|GetB_Color) true)
  (Rendering|Lighting|SetAttenuationRadius (Variables|Default|GetLight_RED) (Variables|Default|GetAttenuation%20Radious))
  (Rendering|Lighting|SetOuterConeAngle (Variables|Default|GetLight_GREEN) (Variables|Default|GetOuter%20Cone%20Angle))
  (Rendering|Lighting|SetInnerConeAngle (Variables|Default|GetLight_GREEN) (Variables|Default|GetInner%20Cone%20Angle))
  (switch int (Variables|Default|GetPick%20Caustic)
    (:2
      (Rendering|Components|Light|SetLightFunctionMaterial (Variables|Default|GetLight_RED) "/Game/CardinalGems/Materials/Mesh_Specific/MI_Caustics_004.MI_Caustics_004")
      (Rendering|Components|Light|SetLightFunctionMaterial (Variables|Default|GetLight_GREEN) "/Game/CardinalGems/Materials/Mesh_Specific/MI_Caustics_005.MI_Caustics_005")
      (Rendering|Components|Light|SetLightFunctionMaterial (Variables|Default|GetLIGHT_Blue) "/Game/CardinalGems/Materials/Mesh_Specific/MI_Caustics_006.MI_Caustics_006"))
    (:3
      (Rendering|Components|Light|SetLightFunctionMaterial (Variables|Default|GetLight_RED) "/Game/CardinalGems/Materials/Mesh_Specific/MI_Caustics_007.MI_Caustics_007")
      (Rendering|Components|Light|SetLightFunctionMaterial (Variables|Default|GetLight_GREEN) "/Game/CardinalGems/Materials/Mesh_Specific/MI_Caustics_008.MI_Caustics_008")
      (Rendering|Components|Light|SetLightFunctionMaterial (Variables|Default|GetLIGHT_Blue) "/Game/CardinalGems/Materials/Mesh_Specific/MI_Caustics_009.MI_Caustics_009"))))